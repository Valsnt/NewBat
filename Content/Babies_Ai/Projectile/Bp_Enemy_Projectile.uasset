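; Enemy projectile Blueprint that damages the player on impact.
; Sphere hit events check the struck component's tags: "ground" spawns a BP_ProjectileTrail at the sphere's location, while "Player" casts the hit actor to DadPawn and calls TakeAwayHealth.
; The projectile then destroys itself, as it does on any other hit, except when the DadPawn cast fails, which leaves it alive.
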(event OnComponentBeginOverlap(Sphere)
  (params (OverlappedComponent :type Primitive%20Component%20Object%20Reference) (OtherActor :type Actor%20Object%20Reference) (OtherComp :type Primitive%20Component%20Object%20Reference) (OtherBodyIndex :type Integer) (bFromSweep :type Boolean) (SweepResult :type Hit%20Result%20Structure%20%28by%20ref%29)))

(event OnComponentHit(Sphere)
  (params (HitComponent :type Primitive%20Component%20Object%20Reference) (OtherActor :type Actor%20Object%20Reference) (OtherComp :type Primitive%20Component%20Object%20Reference) (NormalImpulse :type Vector :default "0, 0, 0") (Hit :type Hit%20Result%20Structure%20%28by%20ref%29))
  (if (Components|ComponentHasTag OtherComp "ground")
    (Game|SpawnActorfromClass "/Game/Babies_Ai/Projectile/BP_ProjectileTrail.BP_ProjectileTrail_C" (Math|Conversions|ToTransform(Vector) (Transformation|GetWorldLocation (Variables|Default|GetSphere))) "Undefined" 0 0)
    (elif (Components|ComponentHasTag OtherComp "Player")
      (bind _asdad_pawn (Utilities|Casting|CastToDadPawn OtherActor))
      (Default|TakeAwayHealth _asdad_pawn 2.0)))
  (Actor|DestroyActor))

(event EventBeginPlay)

(event Collision|EventActorBeginOverlap
  (params (OtherActor :type Actor%20Object%20Reference)))

(event EventTick
  (params (DeltaSeconds :type Float%20%28single-precision%29)))

(fn ConstructionScript)